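; Bamboo platform trap that gives way when BP_KitsuneNinjaPrincess overlaps its trigger Box.
; The overlap plays a Timeline driving the root's world roll, then disables collision on the box and bamboo meshes and hides the meshes.
; A four-second timer calls Reset, which restores collision but sets mesh visibility to false again, leaving the platform invisible.
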(event OnComponentBeginOverlap(Box)
  (params (OverlappedComponent :type Primitive%20Component%20Object%20Reference) (OtherActor :type Actor%20Object%20Reference) (OtherComp :type Primitive%20Component%20Object%20Reference) (OtherBodyIndex :type Integer) (bFromSweep :type Boolean) (SweepResult :type Hit%20Result%20Structure%20%28by%20ref%29))
  (bind _sm_bamsolo_mid5 (Variables|Default|GetSM_BamSolo_Mid5))
  (Utilities|Casting|CastToBP_KitsuneNinjaPrincess OtherActor)
  (bind _newtrack_0 (Timeline|Timeline PlayFromStart)
    (:Update
      (Transformation|SetWorldRotation (Variables|Default|GetDefaultSceneRoot) (Math|Rotator|MakeRotator _newtrack_0 0.0 0.0) false false))
    (:Finished
      (Collision|SetCollisionEnabled _sm_bamsolo_mid5 "NoCollision")
      (Rendering|SetVisibility _sm_bamsolo_mid5 false false)
      (Utilities|Time|SetTimerbyEvent (delegate Custom|Reset) 4.0))))

(event Custom|Reset
  (bind _sm_bamsolo_mid5 (Variables|Default|GetSM_BamSolo_Mid5))
  (Collision|SetCollisionEnabled _sm_bamsolo_mid5 "QueryAndPhysics")
  (Collision|SetCollisionEnabled (Variables|Default|GetBox) "QueryOnly")
  (Rendering|SetVisibility _sm_bamsolo_mid5 false false))

(event EventBeginPlay)

(event Collision|EventActorBeginOverlap
  (params (OtherActor :type Actor%20Object%20Reference)))

(event EventTick
  (params (DeltaSeconds :type Float%20%28single-precision%29)))

(fn ConstructionScript)